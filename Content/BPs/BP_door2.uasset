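; BP_door2 is an interactable door that swings open and closed, with opening gated by a HasKey flag.
; A Box overlap enables interaction and registers the door as the third-person character's LastInteractObj.
; Interact alternates through a FlipFlop between playing and reversing a Timeline that drives mesh yaw, with HasOpen tracking the state.
; NewFunction, Soma and NewMacro are small helpers that the event graph does not use.
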(event `self.Box.OnComponentBeginOverlap`
  (params (OverlappedComponent :type "PrimitiveComponent Object Reference") (OtherActor :type "Actor Object Reference") (OtherComp :type "PrimitiveComponent Object Reference") (OtherBodyIndex :type Integer) (bFromSweep :type Boolean) (SweepResult :type "HitResult Structure (by ref)"))
  ;[1 1 1] EnterCollision
  (bind _asbp_third_person_character (cast `/Game/ThirdPerson/Blueprints/BP_ThirdPersonCharacter` OtherActor))
  (set `/Game/ThirdPerson/Blueprints/BP_ThirdPersonCharacter.LastInteractObj` self _asbp_third_person_character)
  (set `self.CanInteract?` true))

(event `self.Box.OnComponentEndOverlap`
  (params (OverlappedComponent :type "PrimitiveComponent Object Reference") (OtherActor :type "Actor Object Reference") (OtherComp :type "PrimitiveComponent Object Reference") (OtherBodyIndex :type Integer))
  ;[1 1 1] ExitCollision
  (cast `/Game/ThirdPerson/Blueprints/BP_ThirdPersonCharacter` OtherActor)
  (set `self.CanInteract?` false))

(event `/Game/BPs/Interact_Interface.Interact`
  ;[1 1 1] Interact
  (if (`self.CanInteract?`)
    (`/Engine/EditorBlueprintResources/StandardMacros.FlipFlop`
      (:`A`
        (if (`self.HasKey?`)
          (if (not (`self.HasOpen?`))
            (bind (_direction _doormovement) (`Timeline|Timeline` :!via `PlayFromStart` :!label _label)
              (:`Update`
                (`SceneComponent.K2_SetRelativeRotation` (`self.StaticMesh`) (`KismetMathLibrary.MakeRotator` 0.0 0.0 _doormovement) false false))
              (:`Finished`
                (set `self.HasOpen?` (> _doormovement 0.0)))))))
      (:`B`
        (if (`self.HasOpen?`)
          (goto _label :!via `ReverseFromEnd`))))))

(fn `NewFunction`
  (if (`self.HasOpen?`)
    (`SceneComponent.K2_AddWorldOffset` (`self.Box`) (0.0 0.0 0.0) false false)))

(fn `Soma`
  (params (NewParam :type "Float (double-precision)") (NewParam1 :type "Vector Structure"))
  (returns (NewParam2 :type "Vector Structure"))
  (return (* NewParam NewParam1)))

(fn `UserConstructionScript`)