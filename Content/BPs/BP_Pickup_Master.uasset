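; BP_Pickup_Master is a base pickup actor the player character can interact with while inside its Sphere collision.
; Entering the sphere registers the pickup as the character's LastInteractObj and sets CanInteract, and leaving clears only that flag.
; Interact, when allowed, calls the empty Body event, apparently a hook for child pickups, then destroys the actor.
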(event `self.Sphere.OnComponentBeginOverlap`
  (params (OverlappedComponent :type "PrimitiveComponent Object Reference") (OtherActor :type "Actor Object Reference") (OtherComp :type "PrimitiveComponent Object Reference") (OtherBodyIndex :type Integer) (bFromSweep :type Boolean) (SweepResult :type "HitResult Structure (by ref)"))
  ;[1 1 1] Enter Collision
  (bind _asbp_third_person_character (cast `/Game/ThirdPerson/Blueprints/BP_ThirdPersonCharacter` OtherActor)
    (:`then`
      (set `/Game/ThirdPerson/Blueprints/BP_ThirdPersonCharacter.LastInteractObj` self _asbp_third_person_character)
      (set `self.CanInteract?` true))
    (:`CastFailed`
      (`KismetSystemLibrary.PrintString` "ERROR"))))

(event `self.Sphere.OnComponentEndOverlap`
  (params (OverlappedComponent :type "PrimitiveComponent Object Reference") (OtherActor :type "Actor Object Reference") (OtherComp :type "PrimitiveComponent Object Reference") (OtherBodyIndex :type Integer))
  ;[1 1 1] Exit Collision
  (cast `/Game/ThirdPerson/Blueprints/BP_ThirdPersonCharacter` OtherActor)
  (set `self.CanInteract?` false))

(event `/Game/BPs/Interact_Interface.Interact`
  (if (`self.CanInteract?`)
    (`self.Body`)
    (`self.K2_DestroyActor`)
    (`KismetSystemLibrary.PrintString` "Destroy")))

(event `Body`)

(fn `UserConstructionScript`)